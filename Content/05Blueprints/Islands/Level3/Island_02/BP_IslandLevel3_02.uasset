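; A level 3 island the player's ship can visit and plunder, with a random name and fixed loot and attack values set at BeginPlay.
; Entering its sphere as a "Player"-tagged component creates and opens the island's loot widget; leaving closes it through a widget class lookup.
; The IslandPlundered event flags the island as looted and reveals the boiler smoke effect, which starts hidden.
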(event OnComponentEndOverlap(Sphere)
  (params (OverlappedComponent :type Primitive%20Component%20Object%20Reference) (OtherActor :type Actor%20Object%20Reference) (OtherComp :type Primitive%20Component%20Object%20Reference) (OtherBodyIndex :type Integer))
  ;[0 0 0] When player leaves collider call "Close Loot Menu"
  ;;[0 0.3864 1] If a component (the ship) has the tag "Player" THEN do thing.
  (if (Components|ComponentHasTag OtherComp "Player")
    ;;[1 0.7722 0] Get the coresponding widget and call "Close Loot Menu"
    (bind _foundwidgets (Widget|GetAllWidgetsOfClass "/Game/05Blueprints/Islands/Level3/Island_02/BP_IslandLootWidgetLvl3_02.BP_IslandLootWidgetLvl3_02_C" true))
    (Default|Level3IslandCloseLootMenu _foundwidgets)))

(event OnComponentBeginOverlap(Sphere)
  (params (OverlappedComponent :type Primitive%20Component%20Object%20Reference) (OtherActor :type Actor%20Object%20Reference) (OtherComp :type Primitive%20Component%20Object%20Reference) (OtherBodyIndex :type Integer) (bFromSweep :type Boolean) (SweepResult :type Hit%20Result%20Structure%20%28by%20ref%29))
  ;[0 0 0] When a player enters collider call "Open Loot Menu"
  ;;[0 0.3864 1] If a component (the ship) has the tag "Player" THEN do thing.
  (if (Components|ComponentHasTag OtherComp "Player")
    ;;[1 0.7722 0] Create the loot island widget and call "Open Loot Menu"
    (bind _returnvalue (UserInterface|CreateWidget "/Game/05Blueprints/Islands/Level3/Island_02/BP_IslandLootWidgetLvl3_02.BP_IslandLootWidgetLvl3_02_C"))
    (UserInterface|Viewport|AddtoViewport _returnvalue 0)
    (bind _foundwidgets (Widget|GetAllWidgetsOfClass "/Game/05Blueprints/Islands/Level3/Island_02/BP_IslandLootWidgetLvl3_02.BP_IslandLootWidgetLvl3_02_C" true))
    (Default|Level3IslandOpenLootMenu _foundwidgets)))

(event Custom|IslandPlundered
  ;[0 0 0] When called set "IslandPlundered" to true
  (Variables|Default|SetIslandPlundered? true)
  (Development|PrintString "Island plundered")
  (Rendering|SetVisibility (Variables|Default|GetP_BoilerSmoke) true false))

(event EventBeginPlay
  ;[0 0 0] At play set the Island variables.
  (Rendering|SetVisibility (Variables|Default|GetP_BoilerSmoke) false false)
  ;;[1 0.8304 0] Set the name of the island from a list of options.
  (Variables|Default|SetIslandName (.OutItem (Utilities|Array|Random (Variables|Default|GetLevel1IslandNames))))
  ;;[1 0.8536 0] Set the level of the island.
  (Variables|Default|SetIslandLevel 3)
  ;;[1 0.84 0] Set the loot reward from the island.
  (Variables|Default|SetIslandLoot 15)
  ;;[1 0.9832 0] Set the attack power of the island
  (Variables|Default|SetIslandAttackPower 5)
  ;;[1 0.8855 0] Set the island to not yet plundered.
  (Variables|Default|SetIslandPlundered? false))

(fn ConstructionScript)