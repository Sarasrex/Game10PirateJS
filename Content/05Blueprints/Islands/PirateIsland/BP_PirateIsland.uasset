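; BP_PirateIsland is an island actor that opens and closes a loot menu as the player's ship enters and leaves its range.
; Sphere overlap events filter on the overlapping component's "Player" tag, then find existing top-level BP_PirateIslandWidget instances and call their open or close menu functions.
; The widget must already exist in the viewport, as the create-and-add nodes here are unconnected.
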(event OnComponentEndOverlap(Sphere)
  (params (OverlappedComponent :type Primitive%20Component%20Object%20Reference) (OtherActor :type Actor%20Object%20Reference) (OtherComp :type Primitive%20Component%20Object%20Reference) (OtherBodyIndex :type Integer))
  ;[0 0 0] When player leaves collider call "Close Loot Menu"
  ;;[0 0.3864 1] If a component (the ship) has the tag "Player" THEN do thing.
  (if (Components|ComponentHasTag OtherComp "Player")
    ;;[0.002125 0 1] Get the coresponding widget and call "Close Loot Menu"
    (bind _foundwidgets (Widget|GetAllWidgetsOfClass "/Game/05Blueprints/Islands/PirateIsland/BP_PirateIslandWidget.BP_PirateIslandWidget_C" true))
    (Default|PirateIslandCloseMenu _foundwidgets)))

(event OnComponentBeginOverlap(Sphere)
  (params (OverlappedComponent :type Primitive%20Component%20Object%20Reference) (OtherActor :type Actor%20Object%20Reference) (OtherComp :type Primitive%20Component%20Object%20Reference) (OtherBodyIndex :type Integer) (bFromSweep :type Boolean) (SweepResult :type Hit%20Result%20Structure%20%28by%20ref%29))
  ;[0 0 0] When a player enters collider call "Open Loot Menu"
  ;;[0 0.3864 1] If a component (the ship) has the tag "Player" THEN do thing.
  (if (Components|ComponentHasTag OtherComp "Player")
    ;;[0.002125 0 1] Create the loot island widget and call "Open Loot Menu"
    (bind _foundwidgets (Widget|GetAllWidgetsOfClass "/Game/05Blueprints/Islands/PirateIsland/BP_PirateIslandWidget.BP_PirateIslandWidget_C" true))
    (Default|PirateIslandOpenMenu _foundwidgets)))

(event EventBeginPlay)

(fn ConstructionScript)